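; Stationary enemy turret that continuously aims at the player and fires projectiles at regular intervals.
; Tick snaps the actor's full rotation to look at PlayerRef, which is not assigned in these graphs.
; A looping timer started on BeginPlay plays a grenadier throw animation, then after a short delay spawns BP_BulletEnnemy at the actor's transform, so shots follow its current facing.
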(event `self.ReceiveBeginPlay`
  (`KismetSystemLibrary.K2_SetTimerDelegate` (delegate `Fire`) 1.5 true)
  (`parent.ReceiveBeginPlay`))

(event `Fire`
  (`SkeletalMeshComponent.PlayAnimation` (`self.Mesh`) "/Game/CityofBrass_Enemies/Meshes/Enemy/Grenadier/Animation/Grenadier_Attack_Throw.Grenadier_Attack_Throw" false)
  (`KismetSystemLibrary.Delay` 0.8)
  (`|SpawnActorFromClass` "/Game/Ennemy/BP_BulletEnnemy.BP_BulletEnnemy_C" (`self.GetTransform`) "Undefined" "MultiplyWithRoot" null null))

(event `self.ReceiveTick`
  (params (DeltaSeconds :type "Float (single-precision)"))
  (`self.K2_SetActorRotation` (`KismetMathLibrary.FindLookAtRotation` (`self.K2_GetActorLocation`) (`self.K2_GetActorLocation` (`self.Player ref`)))))

(fn `UserConstructionScript`
  (`parent.UserConstructionScript`))