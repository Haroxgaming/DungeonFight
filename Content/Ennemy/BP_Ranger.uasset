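; BP_Ranger is a ranged enemy that alternates between wandering and shooting at the player.
; From BeginPlay, MoveAndFire sends it via AIMoveTo to a random reachable point within a fixed radius.
; On arrival it pauses, turns to face PlayerRef, spawns a BP_BulletEnnemy at its own transform, waits, then calls itself again.
; Only a successful move continues the loop, as the failure path is unhandled.
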(event `self.ReceiveBeginPlay`
  (`self.Move and fire`)
  (`parent.ReceiveBeginPlay`))

(event `Move and fire`
  (`|AIMoveTo` (`PawnMovementComponent.GetPawnOwner` (`self.CharacterMovement`)) (`NavigationSystemV1.K2_GetRandomReachablePointInRadius` (`self.K2_GetActorLocation`) 500.0 null null) null
    (:`OnSuccess`
      (`KismetSystemLibrary.Delay` 0.5)
      (`self.K2_SetActorRotation` (`KismetMathLibrary.FindLookAtRotation` (`self.K2_GetActorLocation`) (`self.K2_GetActorLocation` (`self.Player ref`))))
      (`|SpawnActorFromClass` "/Game/Ennemy/BP_BulletEnnemy.BP_BulletEnnemy_C" (`self.GetTransform`) "Undefined" "MultiplyWithRoot" null null)
      (`KismetSystemLibrary.Delay` 1.0)
      (`self.Move and fire`))))

(fn `UserConstructionScript`
  (`parent.UserConstructionScript`))