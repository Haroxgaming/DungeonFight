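; BP_Rusher is an enemy that continuously chases the player and deals repeated damage at close range.
; Tick issues a simple move to PlayerRef's location.
; Entering the Attack component sets InZone and fires a DoOnce-gated damage message to the player, without checking which actor overlapped.
; After a short delay, the gate resets and Damaging calls itself, repeating until an end overlap clears InZone.
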(event `self.ReceiveBeginPlay`
  (`parent.ReceiveBeginPlay`))

(event `self.ReceiveActorBeginOverlap`
  (params (OtherActor :type "Actor Object Reference"))
  (`parent.ReceiveActorBeginOverlap` OtherActor))

(event `self.ReceiveTick`
  (params (DeltaSeconds :type "Float (single-precision)"))
  (bind _output_get (set `self.Player location` (`self.K2_GetActorLocation` (`self.Player ref`))))
  (`AIBlueprintHelperLibrary.SimpleMoveToLocation` (`self.GetController`) _output_get))

(event `Damaging`
  (if (`self.InZone`)
    (`/Engine/EditorBlueprintResources/StandardMacros.DoOnce` false :!label _label
      (:`Completed`
        (message `/Game/ThirdPerson/Blueprints/BPI_Bullet.DamagePlayer` (`self.Player ref`))
        (`KismetSystemLibrary.Delay` 1.0)
        (`|ExecutionSequence`
          (:`then_0`
            (goto _label :!via `Reset`))
          (:`then_1`
            (`self.Damaging`)))))))

(event `self.Attack.OnComponentBeginOverlap`
  (params (OverlappedComponent :type "PrimitiveComponent Object Reference") (OtherActor :type "Actor Object Reference") (OtherComp :type "PrimitiveComponent Object Reference") (OtherBodyIndex :type Integer) (bFromSweep :type Boolean) (SweepResult :type "HitResult Structure (by ref)"))
  (set `self.InZone` true)
  (goto _label))

(event `self.Attack.OnComponentEndOverlap`
  (params (OverlappedComponent :type "PrimitiveComponent Object Reference") (OtherActor :type "Actor Object Reference") (OtherComp :type "PrimitiveComponent Object Reference") (OtherBodyIndex :type Integer))
  (set `self.InZone` false))

(fn `UserConstructionScript`
  (`parent.UserConstructionScript`))