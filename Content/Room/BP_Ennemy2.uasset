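; BP_Ennemy2 is a room Blueprint that defines a set of enemy spawns for the game.
; Its SpawnEnnemy event spawns actors at the Spawn1, Spawn2 and Spawn3 transforms, passing itself to each as RoomRef.
; The first and third spawns are BP_Ranger, while the second shows no class.
; BeginPlay is disabled and the construction script only calls its parent.
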(event `self.SpawnEnnemy`
  (`|SpawnActorFromClass` "/Game/Ennemy/BP_Ranger.BP_Ranger_C" (`SceneComponent.K2_GetComponentToWorld` (`self.Spawn1`)) "Undefined" "MultiplyWithRoot" null self null)
  (`|SpawnActorFromClass` "/Game/Ennemy/BP_Rusher.BP_Rusher_C" (`SceneComponent.K2_GetComponentToWorld` (`self.Spawn2`)) "Undefined" "MultiplyWithRoot" null self null)
  (`|SpawnActorFromClass` "/Game/Ennemy/BP_Ranger.BP_Ranger_C" (`SceneComponent.K2_GetComponentToWorld` (`self.Spawn3`)) "Undefined" "MultiplyWithRoot" null self null))

(fn `UserConstructionScript`
  (`parent.UserConstructionScript`))