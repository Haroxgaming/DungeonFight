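; BP_Object is a pickup that is either a bomb or a gold coin, with mesh and scale chosen by its Object type.
; The construction script applies that look, and if Random is set, BeginPlay re-rolls the type, favoring gold three to one, and reapplies it.
; When the third-person character overlaps its sphere, it passes the type to the character's AddObject and destroys itself.
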(event `self.ReceiveBeginPlay`
  (bind _staticmesh (`self.StaticMesh`))
  (if (`self.Random`)
    (bind _output_get (set `self.Object` (select `int` (`KismetMathLibrary.RandomIntegerInRange` 0 3) :`0` "NewEnumerator0" :`1` "NewEnumerator2" :`2` "NewEnumerator2" :`3` "NewEnumerator2" :!type "/Game/Object/E_Object Enum")))
    (`StaticMeshComponent.SetStaticMesh` _staticmesh (select `/Game/Object/E_Object` _output_get :`NewEnumerator0` "/Game/Asset/black-handbomb.black-handbomb" :`NewEnumerator2` "/Game/Asset/coin_coin.coin_coin" :!type "StaticMesh Object Reference"))
    (`SceneComponent.SetWorldScale3D` _staticmesh (select `/Game/Object/E_Object` _output_get :`NewEnumerator0` (0.05 0.05 0.05) :`NewEnumerator2` (1.1 1.1 1.1) :!type "Vector Structure"))))

(event `self.Sphere.OnComponentBeginOverlap`
  (params (OverlappedComponent :type "PrimitiveComponent Object Reference") (OtherActor :type "Actor Object Reference") (OtherComp :type "PrimitiveComponent Object Reference") (OtherBodyIndex :type Integer) (bFromSweep :type Boolean) (SweepResult :type "HitResult Structure (by ref)"))
  (bind _asbp_third_person_character (cast `/Game/ThirdPerson/Blueprints/BP_ThirdPersonCharacter` OtherActor))
  (`/Game/ThirdPerson/Blueprints/BP_ThirdPersonCharacter.Add Object` _asbp_third_person_character (`self.Object`))
  (`self.K2_DestroyActor`))

(fn `UserConstructionScript`
  (bind _staticmesh (`self.StaticMesh`))
  (bind _object (`self.Object`))
  (`StaticMeshComponent.SetStaticMesh` _staticmesh (select `/Game/Object/E_Object` _object :`NewEnumerator0` "/Game/Asset/black-handbomb.black-handbomb" :`NewEnumerator2` "/Game/Asset/coin_coin.coin_coin" :!type "StaticMesh Object Reference"))
  (`SceneComponent.SetWorldScale3D` _staticmesh (select `/Game/Object/E_Object` _object :`NewEnumerator0` (0.05 0.05 0.05) :`NewEnumerator2` (1.1 1.1 1.1) :!type "Vector Structure")))