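; BP_ShopItem is a shop pickup that sells one weapon upgrade for a gold cost shown on its text render.
; BeginPlay picks the sprite from the Upgrade enum, while the construction script also previews the price in the editor.
; When the third-person character overlaps its sphere with enough gold, it deducts the cost, updates the HUD, sets the matching upgrade flag on the player and destroys itself.
; Accepted and refused payments each play their own sound.
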(event `self.ReceiveBeginPlay`
  (`TextRenderComponent.K2_SetText` (`self.TextRender`) (`KismetTextLibrary.Conv_IntToText` (`self.Cost`)))
  (`PaperSpriteComponent.SetSprite` (`self.PaperSprite`) (select `/Game/Object/E_UpgradeListe` (`self.Upgrade`) :`NewEnumerator0` "/Game/Object/Image/Explosion_Sprite.Explosion_Sprite" :`NewEnumerator1` "/Game/Object/Image/Spread_Sprite.Spread_Sprite" :`NewEnumerator2` "/Game/Object/Image/Lateral_Sprite.Lateral_Sprite" :`NewEnumerator3` "/Game/Object/Image/Behind_Sprite.Behind_Sprite" :!type "PaperSprite Object Reference")))

(event `Modification`
  (bind _player_ref (`self.Player ref`))
  (switch `/Game/Object/E_UpgradeListe` (`self.Upgrade`)
    (:`NewEnumerator0`
      (set `/Game/ThirdPerson/Blueprints/BP_ThirdPersonCharacter.Explosion` true _player_ref))
    (:`NewEnumerator1`
      (set `/Game/ThirdPerson/Blueprints/BP_ThirdPersonCharacter.DiagonalForward` true _player_ref))
    (:`NewEnumerator2`
      (set `/Game/ThirdPerson/Blueprints/BP_ThirdPersonCharacter.Lateral` true _player_ref))
    (:`NewEnumerator3`
      (set `/Game/ThirdPerson/Blueprints/BP_ThirdPersonCharacter.Behind` true _player_ref))))

(event `self.Sphere.OnComponentBeginOverlap`
  (params (OverlappedComponent :type "PrimitiveComponent Object Reference") (OtherActor :type "Actor Object Reference") (OtherComp :type "PrimitiveComponent Object Reference") (OtherBodyIndex :type Integer) (bFromSweep :type Boolean) (SweepResult :type "HitResult Structure (by ref)"))
  (bind _player_ref (`self.Player ref`))
  (bind _asbp_third_person_character (cast `/Game/ThirdPerson/Blueprints/BP_ThirdPersonCharacter` OtherActor))
  (set `self.Player ref` _asbp_third_person_character)
  (if (>= (`/Game/ThirdPerson/Blueprints/BP_ThirdPersonCharacter.Gold` _asbp_third_person_character) (`self.Cost`))
    (`GameplayStatics.PlaySound2D` "/Game/SoundDesign/Upgrade/SC_PaimentAccepter.SC_PaimentAccepter" 1.0 1.0 0.0 null null)
    (bind _output_get (set `/Game/ThirdPerson/Blueprints/BP_ThirdPersonCharacter.Gold` (- (`/Game/ThirdPerson/Blueprints/BP_ThirdPersonCharacter.Gold` _player_ref) (`self.Cost`)) _player_ref))
    (`/Game/UI/WBP_HUD.Lose Gold` (`/Game/ThirdPerson/Blueprints/BP_ThirdPersonCharacter.HUD Ref` _player_ref) _output_get)
    (`self.Modification`)
    (`self.K2_DestroyActor`)
    (else
      (`GameplayStatics.PlaySound2D` "/Game/SoundDesign/Upgrade/SC_PaimentRefuser.SC_PaimentRefuser" 1.0 1.0 0.0 null null))))

(fn `UserConstructionScript`
  (`TextRenderComponent.K2_SetText` (`self.TextRender`) (`KismetTextLibrary.Conv_IntToText` (`self.Cost`))))