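; Enemy bullet actor that damages the player on overlap and destroys itself when it hits something.
; BeginPlay records the start location, converts Range from meters to centimeters and plays a 2D firing sound.
; Tick shrinks the mesh as it travels past a short initial distance, then destroys the bullet at maximum range.
; Overlaps send DamagePlayerMessage to the other actor without checking what it is.
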(event `self.ReceiveTick`
  (params (DeltaSeconds :type "Float (single-precision)"))
  (bind _range (`self.Range`))
  (bind _returnvalue (`KismetMathLibrary.Vector_Distance` (`self.Start location`) (`self.K2_GetActorLocation`)))
  (if (>= _returnvalue _range)
    (`self.K2_DestroyActor`)
    (elif (>= _returnvalue 300.0)
      (`SceneComponent.SetWorldScale3D` (`self.Mesh`) (`KismetMathLibrary.Conv_DoubleToVector` (/ (- 1.0 (/ (- _returnvalue 300.0) (- _range 300.0))) 2.0))))))

(event `self.ReceiveBeginPlay`
  (set `self.Start location` (`self.K2_GetActorLocation`))
  (set `self.Range` (* (`self.Range`) 100.0))
  (`GameplayStatics.PlaySound2D` "/Game/SoundDesign/TirEnnemi/SC_TirEnnemi.SC_TirEnnemi" 1.0 1.0 0.0 null null))

(event `self.Collide.OnComponentBeginOverlap`
  (params (OverlappedComponent :type "PrimitiveComponent Object Reference") (OtherActor :type "Actor Object Reference") (OtherComp :type "PrimitiveComponent Object Reference") (OtherBodyIndex :type Integer) (bFromSweep :type Boolean) (SweepResult :type "HitResult Structure (by ref)"))
  (message `/Game/ThirdPerson/Blueprints/BPI_Bullet.DamagePlayer` OtherActor)
  (`self.K2_DestroyActor`))

(event `self.Mesh.OnComponentHit`
  (params (HitComponent :type "PrimitiveComponent Object Reference") (OtherActor :type "Actor Object Reference") (OtherComp :type "PrimitiveComponent Object Reference") (NormalImpulse :type "Vector Structure") (Hit :type "HitResult Structure (by ref)"))
  (`self.K2_DestroyActor`))

(fn `UserConstructionScript`)