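; BP_GemShop is a world shop item that the player buys with gems, shown with the Explosion sprite and a price text.
; Shortly after BeginPlay it destroys itself if the player's save already has Explosion, otherwise it sets the sprite and cost.
; Overlapping its sphere with enough gems deducts the cost, calls AchatGem on the player and destroys the shop.
; The construction script also writes the cost to the text.
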(event `self.ReceiveBeginPlay`
  (`KismetSystemLibrary.Delay` 0.2)
  (bind _returnvalue (`GameplayStatics.GetActorOfClass` "/Game/ThirdPerson/Blueprints/BP_ThirdPersonCharacter.BP_ThirdPersonCharacter_C"))
  (bind _output_get (set `self.Player ref` _returnvalue))
  (if (`/Game/ThirdPerson/Blueprints/SG_Save.Explosion` (`/Game/ThirdPerson/Blueprints/BP_ThirdPersonCharacter.As SG Save` _output_get))
    (`self.K2_DestroyActor`)
    (else
      (`TextRenderComponent.K2_SetText` (`self.TextRender`) (`KismetTextLibrary.Conv_IntToText` (`self.Cost`)))
      (`PaperSpriteComponent.SetSprite` (`self.PaperSprite`) "/Game/Object/Image/Explosion_Sprite.Explosion_Sprite"))))

(event `self.Sphere.OnComponentBeginOverlap`
  (params (OverlappedComponent :type "PrimitiveComponent Object Reference") (OtherActor :type "Actor Object Reference") (OtherComp :type "PrimitiveComponent Object Reference") (OtherBodyIndex :type Integer) (bFromSweep :type Boolean) (SweepResult :type "HitResult Structure (by ref)"))
  (bind _player_ref (`self.Player ref`))
  (bind _asbp_third_person_character (cast `/Game/ThirdPerson/Blueprints/BP_ThirdPersonCharacter` OtherActor))
  (bind _output_get (set `self.Player ref` _asbp_third_person_character))
  (if (>= (`/Game/ThirdPerson/Blueprints/BP_ThirdPersonCharacter.Gem` _output_get) (`self.Cost`))
    (set `/Game/ThirdPerson/Blueprints/BP_ThirdPersonCharacter.Gem` (- (`/Game/ThirdPerson/Blueprints/BP_ThirdPersonCharacter.Gem` _player_ref) (`self.Cost`)) _player_ref)
    (`/Game/ThirdPerson/Blueprints/BP_ThirdPersonCharacter.Achat gem` _player_ref)
    (`self.K2_DestroyActor`)))

(fn `UserConstructionScript`
  (`TextRenderComponent.K2_SetText` (`self.TextRender`) (`KismetTextLibrary.Conv_IntToText` (`self.Cost`))))