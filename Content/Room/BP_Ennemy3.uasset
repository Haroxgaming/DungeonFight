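; BP_Ennemy3 is a child room Blueprint that runs an encounter of four Rusher enemies.
; BeginPlay sets the remaining-enemy count to four before calling the parent's logic.
; SpawnEnnemy shows magic-circle particles at four spawn points as a brief telegraph, then removes them and spawns a BP_Rusher at each point.
; Each Rusher receives a reference back to the room.
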(event `self.ReceiveBeginPlay`
  (set `self.EnnemyLeft` 4)
  (`parent.ReceiveBeginPlay`))

(event `self.SpawnEnnemy`
  (for _array_element (`|MakeArray` (`self.Spawn1`) (`self.Spawn2`) (`self.Spawn3`) (`self.Spawn4`))
    (bind (_returnvalue_location _returnvalue_rotation) (`KismetMathLibrary.BreakTransform` (`SceneComponent.K2_GetComponentToWorld` _array_element)))
    (bind _returnvalue (`GameplayStatics.SpawnEmitterAtLocation` "/Game/FXVarietyPack/Particles/P_ky_magicCircle1.P_ky_magicCircle1" _returnvalue_location _returnvalue_rotation (0.5 0.5 0.5)))
    (`KismetArrayLibrary.Array_Add` (`self.AllEmiter`) _returnvalue))
  (`KismetSystemLibrary.Delay` 1.5)
  (for _array_element_2 (`self.AllEmiter`)
    (`ActorComponent.K2_DestroyComponent` _array_element_2))
  (`|SpawnActorFromClass` "/Game/Ennemy/BP_Rusher.BP_Rusher_C" (`SceneComponent.K2_GetComponentToWorld` (`self.Spawn1`)) "Undefined" "MultiplyWithRoot" null self null)
  (`|SpawnActorFromClass` "/Game/Ennemy/BP_Rusher.BP_Rusher_C" (`SceneComponent.K2_GetComponentToWorld` (`self.Spawn2`)) "Undefined" "MultiplyWithRoot" null self null)
  (`|SpawnActorFromClass` "/Game/Ennemy/BP_Rusher.BP_Rusher_C" (`SceneComponent.K2_GetComponentToWorld` (`self.Spawn3`)) "Undefined" "MultiplyWithRoot" null self null)
  (`|SpawnActorFromClass` "/Game/Ennemy/BP_Rusher.BP_Rusher_C" (`SceneComponent.K2_GetComponentToWorld` (`self.Spawn4`)) "Undefined" "MultiplyWithRoot" null self null))

(fn `UserConstructionScript`
  (`parent.UserConstructionScript`))