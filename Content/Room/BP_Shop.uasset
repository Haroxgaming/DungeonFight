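; BP_Shop is a shop room that stocks two purchasable upgrade items when play begins.
; It loads the SG_Save save, or creates and saves one if absent, and adds an extra upgrade to the pool when the save's Explosion flag is set.
; It spawns two fixed-cost BP_ShopItem actors with random upgrades, removing the first pick before the second draw.
; Parent BeginPlay runs after spawning.
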(event `self.ReceiveBeginPlay`
  (bind _save_name (`self.Save name`))
  (bind _returnvalue (`GameplayStatics.DoesSaveGameExist` (`self.Save name`)))
  (if _returnvalue
    (bind _returnvalue_2 (`GameplayStatics.LoadGameFromSlot` _save_name))
    (bind _assg_save (cast `/Game/ThirdPerson/Blueprints/SG_Save` _returnvalue_2))
    (bind _output_get (set `self.As SG Save` _assg_save))
    (if (`/Game/ThirdPerson/Blueprints/SG_Save.Explosion` _output_get)
      (`KismetArrayLibrary.Array_AddUnique` (`self.UpgradeCreate`) "NewEnumerator0"))
    (else
      (bind _returnvalue_3 (`GameplayStatics.CreateSaveGameObject` "/Game/ThirdPerson/Blueprints/SG_Save.SG_Save_C"))
      (bind _output_get_2 (set `self.As SG Save` _returnvalue_3))
      (`GameplayStatics.SaveGameToSlot` _output_get_2 _save_name)))
  (bind _output_get_3 (set `self.TempForChange` (`KismetArrayLibrary.Array_Random` (`self.UpgradeCreate`))))
  (`|SpawnActorFromClass` "/Game/Object/BP_ShopItem.BP_ShopItem_C" (`SceneComponent.K2_GetComponentToWorld` (`self.Spawn4`)) "Undefined" "MultiplyWithRoot" null 5 _output_get_3 null)
  (`KismetArrayLibrary.Array_RemoveItem` (`self.UpgradeCreate`) (`self.TempForChange`))
  (`|SpawnActorFromClass` "/Game/Object/BP_ShopItem.BP_ShopItem_C" (`SceneComponent.K2_GetComponentToWorld` (`self.Spawn1`)) "Undefined" "MultiplyWithRoot" null 5 (`KismetArrayLibrary.Array_Random` (`self.UpgradeCreate`)) null)
  (`parent.ReceiveBeginPlay`))

(fn `UserConstructionScript`
  (`parent.UserConstructionScript`))