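; Base room for a grid of linked rooms, with up to four exits that lock while enemies remain.
; Construction script strips the door, trigger and spawn point from sides without a neighbor.
; When unlocked, triggers teleport the player to the neighbor's opposite spawn, move BP_Cam there and call its CheckEnnemy.
; CheckEnnemy sets lock state and door materials, calling SpawnEnnemy on the first locked check, which here only zeroes EnnemyLeft.
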(event `self.ReceiveBeginPlay`
  (bind _returnvalue (`GameplayStatics.GetActorOfClass` "/Game/ThirdPerson/Blueprints/BP_Cam.BP_Cam_C"))
  (set `self.CamRef` _returnvalue)
  (bind _returnvalue_2 (`GameplayStatics.GetActorOfClass` "/Game/ThirdPerson/Blueprints/BP_ThirdPersonCharacter.BP_ThirdPersonCharacter_C"))
  (set `self.Player Ref` _returnvalue_2))

(event `CheckEnnemy`
  (if (<= (`self.EnnemyLeft`) 0)
    (set `self.CanLeftRoom` true)
    (for _array_element (`|MakeArray` (`self.UpDoor`) (`self.LeftDoor`) (`self.DownDoor`) (`self.RightDoor`))
      (`/Engine/EditorBlueprintResources/StandardMacros.IsValid` _array_element
        (:`Is Valid`
          (`PrimitiveComponent.SetMaterial` _array_element 0 "/Game/Asset/colormap.colormap"))))
    (else
      (set `self.CanLeftRoom` false)
      (`/Engine/EditorBlueprintResources/StandardMacros.DoOnce` false
        (:`Completed`
          (for _array_element_2 (`|MakeArray` (`self.UpDoor`) (`self.LeftDoor`) (`self.DownDoor`) (`self.RightDoor`))
            (`/Engine/EditorBlueprintResources/StandardMacros.IsValid` _array_element_2
              (:`Is Valid`
                (`PrimitiveComponent.SetMaterial` _array_element_2 0 "/AnimationSharing/AnimSharingRed.AnimSharingRed"))))
          (`self.SpawnEnnemy`))))))

(event `self.RightBox.OnComponentBeginOverlap`
  (params (OverlappedComponent :type "PrimitiveComponent Object Reference") (OtherActor :type "Actor Object Reference") (OtherComp :type "PrimitiveComponent Object Reference") (OtherBodyIndex :type Integer) (bFromSweep :type Boolean) (SweepResult :type "HitResult Structure (by ref)"))
  (bind _rightroom (`self.RightRoom`))
  (if (`self.CanLeftRoom`)
    (`self.K2_SetActorLocation` (`self.Player Ref`) (`SceneComponent.K2_GetComponentLocation` (`/Game/Room/BP_RoomBase.SpawnLeft` _rightroom)) false false)
    (`/Game/ThirdPerson/Blueprints/BP_Cam.CamDeplacement` (`self.CamRef`) (`SceneComponent.K2_GetComponentLocation` (`/Game/Room/BP_RoomBase.CameraTarget` _rightroom)))
    (`self.CheckEnnemy` _rightroom)))

(event `self.DownBox.OnComponentBeginOverlap`
  (params (OverlappedComponent :type "PrimitiveComponent Object Reference") (OtherActor :type "Actor Object Reference") (OtherComp :type "PrimitiveComponent Object Reference") (OtherBodyIndex :type Integer) (bFromSweep :type Boolean) (SweepResult :type "HitResult Structure (by ref)"))
  (bind _downroom (`self.DownRoom`))
  (if (`self.CanLeftRoom`)
    (`self.K2_SetActorLocation` (`self.Player Ref`) (`SceneComponent.K2_GetComponentLocation` (`/Game/Room/BP_RoomBase.SpawnUp` _downroom)) false false)
    (`/Game/ThirdPerson/Blueprints/BP_Cam.CamDeplacement` (`self.CamRef`) (`SceneComponent.K2_GetComponentLocation` (`/Game/Room/BP_RoomBase.CameraTarget` _downroom)))
    (`self.CheckEnnemy` _downroom)))

(event `SpawnEnnemy`
  (set `self.EnnemyLeft` 0))

(event `self.UpBox.OnComponentBeginOverlap`
  (params (OverlappedComponent :type "PrimitiveComponent Object Reference") (OtherActor :type "Actor Object Reference") (OtherComp :type "PrimitiveComponent Object Reference") (OtherBodyIndex :type Integer) (bFromSweep :type Boolean) (SweepResult :type "HitResult Structure (by ref)"))
  (bind _uproom (`self.UpRoom`))
  (if (`self.CanLeftRoom`)
    (`self.K2_SetActorLocation` (`self.Player Ref`) (`SceneComponent.K2_GetComponentLocation` (`/Game/Room/BP_RoomBase.SpawnDown` _uproom)) false false)
    (`/Game/ThirdPerson/Blueprints/BP_Cam.CamDeplacement` (`self.CamRef`) (`SceneComponent.K2_GetComponentLocation` (`/Game/Room/BP_RoomBase.CameraTarget` _uproom)))
    (`self.CheckEnnemy` _uproom)))

(event `self.LeftBox.OnComponentBeginOverlap`
  (params (OverlappedComponent :type "PrimitiveComponent Object Reference") (OtherActor :type "Actor Object Reference") (OtherComp :type "PrimitiveComponent Object Reference") (OtherBodyIndex :type Integer) (bFromSweep :type Boolean) (SweepResult :type "HitResult Structure (by ref)"))
  (bind _leftroom (`self.LeftRoom`))
  (if (`self.CanLeftRoom`)
    (`self.K2_SetActorLocation` (`self.Player Ref`) (`SceneComponent.K2_GetComponentLocation` (`/Game/Room/BP_RoomBase.SpawnRight` _leftroom)) false false)
    (`/Game/ThirdPerson/Blueprints/BP_Cam.CamDeplacement` (`self.CamRef`) (`SceneComponent.K2_GetComponentLocation` (`/Game/Room/BP_RoomBase.CameraTarget` _leftroom)))
    (`self.CheckEnnemy` _leftroom)))

(fn `UserConstructionScript`
  (`self.RightRoom`
    (:`then`
      _)
    (:`else`
      (`ActorComponent.K2_DestroyComponent` (`self.RightBox`))
      (`ActorComponent.K2_DestroyComponent` (`self.RightDoor`))
      (`ActorComponent.K2_DestroyComponent` (`self.SpawnRight`))))
  (`self.UpRoom`
    (:`then`
      _)
    (:`else`
      (`ActorComponent.K2_DestroyComponent` (`self.UpDoor`))
      (`ActorComponent.K2_DestroyComponent` (`self.UpBox`))
      (`ActorComponent.K2_DestroyComponent` (`self.SpawnUp`))))
  (`self.DownRoom`
    (:`then`
      _)
    (:`else`
      (`ActorComponent.K2_DestroyComponent` (`self.DownDoor`))
      (`ActorComponent.K2_DestroyComponent` (`self.SpawnDown`))
      (`ActorComponent.K2_DestroyComponent` (`self.DownBox`))))
  (`self.LeftRoom`
    (:`then`)
    (:`else`
      (`ActorComponent.K2_DestroyComponent` (`self.LeftDoor`))
      (`ActorComponent.K2_DestroyComponent` (`self.SpawnLeft`))
      (`ActorComponent.K2_DestroyComponent` (`self.LeftBox`)))))