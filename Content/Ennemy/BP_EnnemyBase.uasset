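; BP_EnnemyBase is an enemy base Blueprint that tracks life and dies when it runs out.
; On Damage it subtracts the amount from Life and passes Life and MaxLife to the WBP_EnnemyLifeBar on its widget component.
; When Life reaches zero it calls the Death event, which destroys the actor.
; The death check only runs if the widget cast succeeds, because a failed cast stops the chain.
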(event `/Game/ThirdPerson/Blueprints/BPI_Bullet.Damage`
  (params (Damage :type "Float (double-precision)"))
  (set `self.Life` (- (`self.Life`) Damage))
  (bind _aswbp_ennemy_life_bar (cast `/Game/Ennemy/WBP_EnnemyLifeBar` (`WidgetComponent.GetWidget` (`self.Widget`))))
  (`/Game/Ennemy/WBP_EnnemyLifeBar.Update Life` _aswbp_ennemy_life_bar (`self.Life`) (`self.MaxLife`))
  (if (<= (`self.Life`) 0.0)
    (`self.Death`)))

(event `Death`
  (`self.K2_DestroyActor`))

(fn `UserConstructionScript`)